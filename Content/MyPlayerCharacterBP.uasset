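; Player character Blueprint that handles an over-the-shoulder aim camera with left/right shoulder switching.
; Holding right mouse sets IsAiming, removes camera boom lag and uses Timelines to lerp the camera to the active shoulder's component location; releasing restores lag and returns it to Default.
; Pressing E while aiming flips the CameraShoulder enum and lerps the camera to the other side, printing the side name.
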(event `self.ReceiveBeginPlay`
  (set `self.Camera Shoulder` "NewEnumerator0"))

(event `Key|RightMouseButton`
  (params (Key :type "Key Structure"))
  (bind _cameracomponent (`self.CameraComponent`))
  (bind _cameracomponent_2 (`self.CameraComponent`))
  (bind _cameracomponent_3 (`self.CameraComponent`))
  ;[1 1 1] Camera Lerp
  (:`Pressed`
    (set `self.Is Aiming` true)
    (set `SpringArmComponent.CameraLagSpeed` 0.0 (`self.CameraBoom`))
    (bind (_direction _newtrack_0) (`Timeline|Timeline_0` :!via `PlayFromStart`)
      (:`Update`
        (if (`|EnumEquality` "NewEnumerator0" (`self.Camera Shoulder`))
          (`SceneComponent.K2_SetRelativeLocation` _cameracomponent_3 (`KismetMathLibrary.VLerp` (`SceneComponent.RelativeLocation` _cameracomponent_3) (`SceneComponent.RelativeLocation` (`self.Right Shoulder`)) _newtrack_0) false false)
          (else
            (`SceneComponent.K2_SetRelativeLocation` _cameracomponent (`KismetMathLibrary.VLerp` (`SceneComponent.RelativeLocation` _cameracomponent) (`SceneComponent.RelativeLocation` (`self.Left Shoulder`)) _newtrack_0) false false))))))
  (:`Released`
    (set `self.Is Aiming` false)
    (set `SpringArmComponent.CameraLagSpeed` 10.0 (`self.CameraBoom`))
    (bind (_direction_2 _newtrack_0_2) (`Timeline|Timeline_1` :!via `PlayFromStart`)
      (:`Update`
        (`SceneComponent.K2_SetRelativeLocation` _cameracomponent_2 (`KismetMathLibrary.VLerp` (`SceneComponent.RelativeLocation` _cameracomponent_2) (`SceneComponent.RelativeLocation` (`self.Default `)) _newtrack_0_2) false false)))))

(event `Key|E`
  (params (Key :type "Key Structure"))
  ;[1 1 1] Shoulder Position Switch
  (:`Pressed`
    (if (`self.Is Aiming`)
      (if (`|EnumEquality` "NewEnumerator0" (`self.Camera Shoulder`))
        (`KismetSystemLibrary.PrintString` "Left")
        (bind (_direction _newtrack_0) (`Timeline|Timeline_2` :!via `PlayFromStart`)
          (:`Update`
            (set `self.Camera Shoulder` "NewEnumerator1")
            (`SceneComponent.K2_SetRelativeLocation` (`self.CameraComponent`) (`KismetMathLibrary.VLerp` (`SceneComponent.RelativeLocation` (`self.CameraComponent`)) (`SceneComponent.RelativeLocation` (`self.Left Shoulder`)) _newtrack_0) false false)))
        (else
          (`KismetSystemLibrary.PrintString` "Right")
          (bind (_direction_2 _newtrack_0_2) (`Timeline|Timeline_3` :!via `PlayFromStart`)
            (:`Update`
              (set `self.Camera Shoulder` "NewEnumerator0")
              (`SceneComponent.K2_SetRelativeLocation` (`self.CameraComponent`) (`KismetMathLibrary.VLerp` (`SceneComponent.RelativeLocation` (`self.CameraComponent`)) (`SceneComponent.RelativeLocation` (`self.Right Shoulder`)) _newtrack_0_2) false false))))))))

(fn `UserConstructionScript`)